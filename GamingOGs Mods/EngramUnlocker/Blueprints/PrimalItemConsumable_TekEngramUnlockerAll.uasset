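; Consumable item from the EngramUnlocker mod that unlocks Tek engrams when used.
; On use, it checks that the inventory owner is a ShooterCharacter, then runs cheat console commands.
; A bulk Tek-only engram command comes first, followed by individual unlocks for Genesis Tek items by blueprint path.
; The commands pass no specific player, as the cast only gates execution.
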(event `self.BlueprintUsed`
  (bind _unlock_tek_engrams (`self.Unlock Tek Engrams`))
  ;[1 1 1] Unlocks Tek Engrams
  (set `self.Unlock Tek Engrams` self)
  (cast `ShooterCharacter` (`ActorComponent.GetOwner` (`PrimalItem.OwnerInventory` _unlock_tek_engrams)))
  (`KismetSystemLibrary.ExecuteConsoleCommand` _unlock_tek_engrams "cheat GiveEngramsTekOnly")
  (`KismetSystemLibrary.ExecuteConsoleCommand` _unlock_tek_engrams "cheat unlockengram \"Blueprint'/Game/Genesis/Weapons/TekHandBlades/PrimalItem_WeaponTekClaws.PrimalItem_WeaponTekClaws'\"")
  (`KismetSystemLibrary.ExecuteConsoleCommand` _unlock_tek_engrams "cheat unlockengram \"Blueprint'/Game/Genesis/CoreBlueprints/Items/PrimalItem_Spawner_HoverSkiff.PrimalItem_Spawner_HoverSkiff'\"")
  (`KismetSystemLibrary.ExecuteConsoleCommand` _unlock_tek_engrams "cheat unlockengram \"Blueprint'/Game/Genesis/Dinos/SpaceWhale/PrimalItemArmor_SpaceWhaleSaddle_Tek.PrimalItemArmor_SpaceWhaleSaddle_Tek'\"")
  (`KismetSystemLibrary.ExecuteConsoleCommand` _unlock_tek_engrams "cheat unlockengram \"Blueprint'/Game/Genesis/Weapons/CruiseMissile/PrimalItem_WeaponTekCruiseMissile.PrimalItem_WeaponTekCruiseMissile'\"")
  (`KismetSystemLibrary.ExecuteConsoleCommand` _unlock_tek_engrams "cheat unlockengram \"Blueprint'/Game/Genesis/Items/Armor/PrimalItemArmor_ShoulderCannon.PrimalItemArmor_ShoulderCannon'\""))