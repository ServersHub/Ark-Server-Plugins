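; Zombo mod flying ant (Titanomyrma Soldier) dino character whose attack index 1 spawns a Dodo at its projectile box.
; Possession enables local input: X toggles timeline mesh scaling via CanLayEgg, and holding R boosts fly speed, both through Server-to-Multi event pairs.
; A looping, never-cleared stamina timer resets speed when stamina runs low.
; The floating HUD draws name and level; firework and item-drop logic is unwired.
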(event `self.BPDoAttack`
  (params (AttackIndex :type Integer))
  (if (== AttackIndex 1)
    (`self.FirePro`)))

(event `FirePro`
  (bind _projectilebox (`self.ProjectileBox`))
  (`|SpawnActorFromClass` "/Game/PrimalEarth/Dinos/Dodo/Dodo_Character_BP.Dodo_Character_BP_C" (`KismetMathLibrary.MakeTransform` (`SceneComponent.K2_GetComponentLocation` _projectilebox) (`SceneComponent.K2_GetComponentRotation` _projectilebox)) true))

(event `ON OFF Server`
  (params (Enabled :type Boolean))
  (set `self.CanLayEgg` Enabled false)
  (`self.ON OFF Multi` (`self.CanLayEgg`)))

(event `Boost Server`
  (params (Enabled :type Boolean))
  (set `self.Boost` Enabled false)
  (`self.Boost Multi` (`self.Boost`)))

(event `ON OFF Multi`
  (params (Enabled :type Boolean))
  (if Enabled
    (`self.ScaleUp`)
    (else
      (`self.ScaleDown`))))

(event `Boost Multi`
  (params (Enabled :type Boolean))
  (if Enabled
    (`self.SpeedOn`)
    (else
      (`self.SpeedOFF`))))

(event `Key|X`
  (:`Pressed`
    (`/Engine/EditorBlueprintResources/StandardMacros.FlipFlop`
      (:`A`
        (`self.ON OFF Server` true))
      (:`B`
        (`self.ON OFF Server` false)))))

(event `Key|R` :consume false
  (:`Pressed`
    (`self.Boost Server` true))
  (:`Released`
    (`self.Boost Server` false)))

(event `ScaleUp`
  (bind (_direction _scaleovertime) (`Timeline|ScaleOverTime` :!label _label)
    (:`Update`
      _)
    (:`Finished`
      _))
  (set `self.NewScale` (`KismetMathLibrary.Conv_DoubleToVector` _scaleovertime) false)
  (`SceneComponent.SetRelativeScale3D` (`self.Mesh`) (`self.NewScale`)))

(event `ScaleDown`
  (goto _label :!via `Reverse`))

(event `SpeedOn`
  (bind _asprimalcharacter (cast `PrimalCharacter` (`self.Instigator`)))
  (bind _charactermovement (`Character.CharacterMovement` _asprimalcharacter))
  (set `CharacterMovementComponent.MaxFlySpeed` (+ (`CharacterMovementComponent.MaxFlySpeed` _charactermovement) 500.0) _charactermovement)
  (`KismetSystemLibrary.K2_SetTimerDelegate` (delegate `StamCheck`) 1.0 true))

(event `SpeedOFF`
  (set `CharacterMovementComponent.MaxFlySpeed` 185.0 (`Character.CharacterMovement` (stale `SpeedOn` _asprimalcharacter))))

(event `StamCheck`
  ;[0.255 0 0.00541] StamCheck
  (if (< (`PrimalCharacterStatusComponent.BPGetCurrentStatusValue` (`PrimalCharacter.MyCharacterStatusComponent` (stale `SpeedOn` _asprimalcharacter)) "Stamina") 2.0)
    (`self.SpeedOFF`)))

(fn `BlueprintDrawFloatingHUD`
  (params (HUD :type "ShooterHUD Object Reference") (CenterX :type "Float (double-precision)") (CenterY :type "Float (double-precision)") (DrawScale :type "Float (double-precision)"))
  (bind _returnvalue (* DrawScale 1.0))
  (bind _canvas (`HUD.Canvas` HUD))
  (`Canvas.SetDrawColor` _canvas (`KismetMathLibrary.Conv_LinearColorToColor` (struct :`R` 1.0 :`G` 0.991363 :`A` 0.3)))
  (if (`self.bIsFemale`)
    (set `self.Wild Dino` "Titanomyrma Soldier")
    (else
      (set `self.Wild Dino` "Titanomyrma Soldier")))
  (`Canvas.BPDrawTextCentered` _canvas "/Game/OldAssets/UI/HUD/Roboto18.Roboto18" (`KismetStringLibrary.Concat_StrStr` (`self.Wild Dino`) (`KismetStringLibrary.Concat_StrStr` " - Lvl " (`KismetStringLibrary.Conv_IntToString` (`PrimalCharacterStatusComponent.BaseCharacterLevel` (`self.DinoCharacterStatus_BP_FlyingAnt_C1`))))) CenterX (+ CenterY 80.0) _returnvalue _returnvalue true true))

(fn `OnRep_Boost`)

(fn `OnRep_CanLayEgg`)

(fn `ReceivePossessed`
  (params (NewController :type "Controller Object Reference"))
  (`/Engine/EditorBlueprintResources/ActorMacros.Switch Has Authority`
    (:`Authority`
      _)
    (:`Remote`
      _))
  (if (not (`KismetSystemLibrary.IsDedicatedServer`))
    (bind _returnvalue (`self.GetOwnerController` NewController))
    (if (`Controller.IsLocalController` _returnvalue)
      (`self.EnableInput` _returnvalue))))

(fn `UserConstructionScript`
  (`parent.UserConstructionScript`))