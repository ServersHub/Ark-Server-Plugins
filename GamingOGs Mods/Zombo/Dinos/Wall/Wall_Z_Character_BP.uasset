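; Wall dino character for the Zombo mod that can switch between three static mesh looks and spawn Dodos as an attack.
; Attack index 1 spawns a Dodo_Character_BP at ProjectileBox; an older firework rocket launch is left disconnected.
; Local possession enables input, so X sets CanLayEgg through ONOFFServer and ONOFFMulti, whose looping MultiGate shows the next mesh.
; The floating HUD is hidden and its draw override is empty.
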(event `self.BPDoAttack`
  (params (AttackIndex :type Integer))
  (if (== AttackIndex 1)
    (`self.FirePro`)))

(event `FirePro`
  (bind _projectilebox (`self.ProjectileBox`))
  (`|SpawnActorFromClass` "/Game/PrimalEarth/Dinos/Dodo/Dodo_Character_BP.Dodo_Character_BP_C" (`KismetMathLibrary.MakeTransform` (`SceneComponent.K2_GetComponentLocation` _projectilebox) (`SceneComponent.K2_GetComponentRotation` _projectilebox)) true))

(event `ON OFF Server`
  (params (Enabled :type Boolean))
  (set `self.CanLayEgg` Enabled false)
  (`self.ON OFF Multi` (`self.CanLayEgg`)))

(event `ON OFF Multi`
  (params (Enabled :type Boolean))
  (if Enabled
    (`self.SwitchMesh` 0)))

(event `Key|X`
  (:`Pressed`
    (`self.ON OFF Server` true)))

(event `SwitchMesh`
  (params (Int :type Integer))
  (bind _staticmesh1 (`self.StaticMesh1`))
  (bind _staticmesh2 (`self.StaticMesh2`))
  (bind _staticmesh3 (`self.StaticMesh3`))
  (`|MultiGate` false true
    (:`Out 0`
      (`SceneComponent.SetVisibility` _staticmesh1 false false)
      (`SceneComponent.SetVisibility` _staticmesh2 true false)
      (`SceneComponent.SetVisibility` _staticmesh3 false false))
    (:`Out 1`
      (`SceneComponent.SetVisibility` _staticmesh1 true false)
      (`SceneComponent.SetVisibility` _staticmesh2 false false)
      (`SceneComponent.SetVisibility` _staticmesh3 false false))
    (:`Out 2`
      (`SceneComponent.SetVisibility` _staticmesh1 false false)
      (`SceneComponent.SetVisibility` _staticmesh2 false false)
      (`SceneComponent.SetVisibility` _staticmesh3 true false))))

(fn `BlueprintDrawFloatingHUD`
  (params (HUD :type "ShooterHUD Object Reference") (CenterX :type "Float (double-precision)") (CenterY :type "Float (double-precision)") (DrawScale :type "Float (double-precision)")))

(fn `OnRep_CanLayEgg`)

(fn `ReceivePossessed`
  (params (NewController :type "Controller Object Reference"))
  (`/Engine/EditorBlueprintResources/ActorMacros.Switch Has Authority`
    (:`Authority`
      _)
    (:`Remote`
      _))
  (if (not (`KismetSystemLibrary.IsDedicatedServer`))
    (bind _returnvalue (`self.GetOwnerController` NewController))
    (if (`Controller.IsLocalController` _returnvalue)
      (`self.EnableInput` _returnvalue))))

(fn `UserConstructionScript`
  (`parent.UserConstructionScript`)
  (set `self.bHideFloatingHUD` true))