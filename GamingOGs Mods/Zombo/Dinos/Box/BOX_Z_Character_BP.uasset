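; Rideable-style box dino character for an ARK mod that spawns Dodos as an attack and drops items as "eggs".
; Attack index 1 spawns a Dodo at the ProjectileBox; a firework rocket variant is left disconnected.
; Pressing X, enabled for the local controller on possession, runs server-then-multi events into LayEgg.
; LayEgg passes each ItemSpawn entry through a storage-box inventory, dropping it at a random offset sized by the Poop box.
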(event `self.BPDoAttack`
  (params (AttackIndex :type Integer))
  (if (== AttackIndex 1)
    (`self.FirePro`)))

(event `FirePro`
  (bind _projectilebox (`self.ProjectileBox`))
  (`|SpawnActorFromClass` "/Game/PrimalEarth/Dinos/Dodo/Dodo_Character_BP.Dodo_Character_BP_C" (`KismetMathLibrary.MakeTransform` (`SceneComponent.K2_GetComponentLocation` _projectilebox) (`SceneComponent.K2_GetComponentRotation` _projectilebox)) true))

(event `ON OFF Server`
  (params (Enabled :type Boolean))
  (set `self.CanLayEgg` Enabled false)
  (`self.ON OFF Multi` (`self.CanLayEgg`)))

(event `ON OFF Multi`
  (params (Enabled :type Boolean))
  (if Enabled
    (`self.LayEgg`)))

(event `Key|X`
  (:`Pressed`
    (`self.ON OFF Server` true)))

(event `LayEgg`
  (bind _primalinventorybp_storagebox_small_c1 (`self.PrimalInventoryBP_StorageBox_Small_C1`))
  (bind _primalinventorybp_storagebox_small_c1_2 (`self.PrimalInventoryBP_StorageBox_Small_C1`))
  (bind _poop (`self.Poop`))
  (bind _returnvalue (`SceneComponent.K2_GetComponentRotation` _poop))
  (bind _inventoryitems (`PrimalInventoryComponent.InventoryItems` _primalinventorybp_storagebox_small_c1))
  (bind _item (`KismetArrayLibrary.Array_Get` _inventoryitems))
  (bind _x (.x (`BoxComponent.GetScaledBoxExtent` _poop)))
  (bind _y (.y (`BoxComponent.GetScaledBoxExtent` _poop)))
  (bind _z (.z (`BoxComponent.GetScaledBoxExtent` _poop)))
  (`/Engine/EditorBlueprintResources/StandardMacros.IsValid` _primalinventorybp_storagebox_small_c1_2
    (:`Is Valid`
      (for _array_element (`self.ItemSpawn`)
        (`PrimalItem.AddNewItem` _array_element _primalinventorybp_storagebox_small_c1_2 false false 0.0 false 1)
        (`SceneComponent.SetWorldLocation` _poop (+ (`KismetMathLibrary.MakeVector` (`KismetMathLibrary.RandomFloatInRange` (* _x -1.0) _x) (`KismetMathLibrary.RandomFloatInRange` (* _y -1.0) _y) (`KismetMathLibrary.RandomFloatInRange` (* _z -1.0) _z)) (`self.K2_GetActorLocation`)) false)
        (bind _asprimalitem (castclass `PrimalItem` (`GameplayStatics.GetObjectClass` _item)))
        (bind _returnvalue_2 (`SceneComponent.GetWorldLocation` _poop))
        (`PrimalInventoryComponent.StaticDropNewItem` _primalinventorybp_storagebox_small_c1 self _asprimalitem 0.0 true (`PrimalItem.ItemQuantity` _item) false null _returnvalue true _returnvalue_2 _returnvalue true true false true null (0.0 0.0 0.0) null 0.0)
        (`KismetArrayLibrary.Array_RemoveItem` _inventoryitems _item)))))

(fn `BlueprintDrawFloatingHUD`
  (params (HUD :type "ShooterHUD Object Reference") (CenterX :type "Float (double-precision)") (CenterY :type "Float (double-precision)") (DrawScale :type "Float (double-precision)")))

(fn `OnRep_CanLayEgg`)

(fn `ReceivePossessed`
  (params (NewController :type "Controller Object Reference"))
  (`/Engine/EditorBlueprintResources/ActorMacros.Switch Has Authority`
    (:`Authority`
      _)
    (:`Remote`
      _))
  (if (not (`KismetSystemLibrary.IsDedicatedServer`))
    (bind _returnvalue (`self.GetOwnerController` NewController))
    (if (`Controller.IsLocalController` _returnvalue)
      (`self.EnableInput` _returnvalue))))

(fn `UserConstructionScript`
  (`parent.UserConstructionScript`)
  (set `self.bHideFloatingHUD` true))