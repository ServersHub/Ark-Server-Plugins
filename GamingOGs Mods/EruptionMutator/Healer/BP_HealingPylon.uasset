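; Placeable healing pylon structure that buffs injured same-team dinos within range, overriding one build-placement restriction code.
; After spawn, the server starts a looping timer at the healing interval, skipped for placement previews.
; CheckForDinos uses an octree overlap to find living, damaged allies past their damage cooldown, then applies Buff_HealingPylon to them.
; When targets are found, StartChargeEvent plays Tek portal animations and a timeline-driven charge particle.
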(event Custom|StartChargeEvent
  (bind _mutatorchargeparticle (Variables|Default|GetMutatorChargeParticle))
  (Components|Animation|PlayAnimation (Variables|Default|GetSkeletalMesh1) "/Game/Mods/EruptionMutator/Tek_Portal-Activate.Tek_Portal-Activate" false)
  (Components|Activation|Activate (Variables|Default|GetMutatorChargeParticle) false)
  (bind _chargevalue (Timeline|ChargeTimeline PlayFromStart)
    (:Update
      (Effects|Components|ParticleSystem|SetVectorParameter _mutatorchargeparticle "InnerCircle" _chargevalue))
    (:Finished
      (Components|Activation|Deactivate _mutatorchargeparticle)
      (Components|Animation|PlayAnimation (Variables|Default|GetSkeletalMesh1) "/Game/Mods/EruptionMutator/Tek_Portal-Deactivate.Tek_Portal-Deactivate" false))))

(event EventBeginPlay
  (Utilities|FlowControl|Delay 0.2)
  (if (not (Variables|Default|GetbIsPreviewStructure))
    (Networking|SwitchHasAuthority
      (:Authority
        (Utilities|Time|SetTimerbyEvent (EventDispatchers|CreateEvent self :!event CheckforDinos) (Variables|Healing|GetHealingInterval) true)))))

(fn ConstructionScript
  (|CallParentFunction))

(fn BPIsAllowedtoBuild
  (params (OutPlacementData :type Placement%20Data%20Structure%20%28by%20ref%29) (CurrentAllowedReason :type Integer))
  (return (Math|Integer|SelectInt 1 CurrentAllowedReason (== CurrentAllowedReason -9))))

(fn CheckforDinos
  (bind _founddinos (LocalVariables|GetFoundDinos))
  (bind _returnvalue (Class|VictoryCore|ServerOctreeOverlapActorsClass (Class|Actor|GetWorld) (Transformation|GetActorLocation) (Variables|Healing|GetHealingRange) "DINOPAWNS" "/Script/ShooterGame.PrimalDinoCharacter" false))
  (for _array_element _returnvalue
    (bind _asprimaldinocharacter (Utilities|Casting|CastToPrimalDinoCharacter _array_element))
    (if (> (- (Utilities|Time|GetGameTimeinSeconds) (Variables|/Script/ShooterGame.PrimalCharacter|GetLastHitDamageTime _asprimaldinocharacter)) (Math|Conversions|ToFloat(Integer) (Variables|Default|GetDamageCooldownTime)))
      (bind _returnvalue_2 (Class|PrimalCharacter|GetCharacterStatusComponent _asprimaldinocharacter))
      (if (< (Class|PrimalCharacterStatusComponent|BPGetCurrentStatusValue _returnvalue_2 "Health") (Class|PrimalCharacterStatusComponent|BPGetMaxStatusValue _returnvalue_2 "Health"))
        (if (not (Variables|/Script/ShooterGame.PrimalCharacter|GetbIsDead _asprimaldinocharacter))
          (if (== (Variables|/Script/Engine.Actor|GetTargetingTeam _asprimaldinocharacter) (Variables|Default|GetTargetingTeam))
            (Utilities|Array|Add (LocalVariables|GetFoundDinos) _asprimaldinocharacter))))))
  (if (> (Utilities|Array|Length _founddinos) 0)
    (CallFunction|StartChargeEvent)
    (for _array_element_2 _founddinos
      (Class|PrimalBuff|StaticAddBuff "/Game/Mods/EruptionMutator/Healer/Buff_HealingPylon.Buff_HealingPylon_C" _array_element_2 0 0 false))))