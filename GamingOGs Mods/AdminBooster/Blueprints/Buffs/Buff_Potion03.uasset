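; Potion buff from the AdminBooster mod that hides the instigating shooter character while the buff is active.
; Shortly after BeginPlay, it sets the character hidden in game and plays a sound at its location, but only if a current weapon is valid.
; On destruction it unhides the character under the same weapon check, so a character without a weapon at that moment stays hidden.
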(event `self.ReceiveBeginPlay`
  (bind _instigator (`self.Instigator`))
  ;[1 1 1] Give Buff
  (`KismetSystemLibrary.Delay` 0.2)
  (bind _asshootercharacter (cast `ShooterCharacter` _instigator))
  (`/Engine/EditorBlueprintResources/StandardMacros.IsValid` (`ShooterCharacter.CurrentWeapon` _asshootercharacter)
    (:`Is Valid`
      (`self.SetActorHiddenInGame` _instigator true)
      (`GameplayStatics.PlaySoundAtLocation` "/Game/Mods/AdminBooster/Sounds/wood_wall_sound__1_.wood_wall_sound__1_" (`self.K2_GetActorLocation` _instigator)))))

(event `self.ReceiveDestroyed`
  (bind _instigator (`self.Instigator`))
  ;[1 1 1] Destroy Buff
  (bind _asshootercharacter (cast `ShooterCharacter` _instigator))
  (`/Engine/EditorBlueprintResources/StandardMacros.IsValid` (`ShooterCharacter.CurrentWeapon` _asshootercharacter)
    (:`Is Valid`
      (`self.SetActorHiddenInGame` _instigator false))))

(fn `UserConstructionScript`)