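; GM admin buff that gives its ShooterCharacter god mode and invisibility to enemies through cheat console commands while active.
; On begin, after a short delay and only with a valid current weapon, it enables both cheats and, if Buff_Vanish is present, hides admin tags on GM and Speed buffs, including Zombo variants.
; Destruction reverses the cheats under the same weapon check, but its tag-unhide branches fetch Buff_Vanish before casting and omit Buff_Speed.
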(event `self.ReceiveBeginPlay`
  ;[1 1 1] Buff Effects Begins
  (`KismetSystemLibrary.Delay` 0.2)
  (bind _asshootercharacter (cast `ShooterCharacter` (`self.Instigator`)))
  (`/Engine/EditorBlueprintResources/StandardMacros.IsValid` (`ShooterCharacter.CurrentWeapon` _asshootercharacter)
    (:`Is Valid`
      (`KismetSystemLibrary.ExecuteConsoleCommand` "cheat enemyinvisible true")
      (`KismetSystemLibrary.ExecuteConsoleCommand` "cheat setgodmode true")
      (bind _asprimalcharacter (cast `PrimalCharacter` (`self.GetOwner`)))
      (bind _returnvalue (`PrimalCharacter.HasBuff` _asprimalcharacter "/Game/Mods/AdminBooster/Blueprints/Buffs/Buff_Vanish.Buff_Vanish_C" false))
      (if _returnvalue
        (`|ExecutionSequence`
          (:`then_0`
            (bind _returnvalue_2 (`PrimalCharacter.GetBuff` _asprimalcharacter "Buff_GM_C"))
            (bind _asbuff_gm_c (cast `/GamingOGs Mods/AdminBooster/Blueprints/Buffs/Buff_GM` _returnvalue_2))
            (`SceneComponent.SetHiddenInGame` (`/GamingOGs Mods/AdminBooster/Blueprints/Buffs/Buff_GM.AdminTagBack` _asbuff_gm_c) true false)
            (`SceneComponent.SetHiddenInGame` (`/GamingOGs Mods/AdminBooster/Blueprints/Buffs/Buff_GM.AdminTagFront` _asbuff_gm_c) true false))
          (:`then_1`
            (bind _returnvalue_3 (`PrimalCharacter.GetBuff` _asprimalcharacter "/Game/Mods/AdminBooster/Blueprints/Buffs/Buff_ZomboGM.Buff_ZomboGM_C"))
            (bind _asbuff_zombogm_c (cast `/Game/Mods/AdminBooster/Blueprints/Buffs/Buff_ZomboGM` _returnvalue_3))
            (`SceneComponent.SetHiddenInGame` (`/Game/Mods/AdminBooster/Blueprints/Buffs/Buff_ZomboGM.AdminTagBack` _asbuff_zombogm_c) true false)
            (`SceneComponent.SetHiddenInGame` (`/Game/Mods/AdminBooster/Blueprints/Buffs/Buff_ZomboGM.AdminTagFront` _asbuff_zombogm_c) true false))
          (:`then_2`
            (bind _returnvalue_4 (`PrimalCharacter.GetBuff` _asprimalcharacter "/Game/Mods/AdminBooster/Blueprints/Buffs/Buff_ZomboSpeed.Buff_ZomboSpeed_C"))
            (bind _asbuff_zombospeed_c (cast `/Game/Mods/AdminBooster/Blueprints/Buffs/Buff_ZomboSpeed` _returnvalue_4))
            (`SceneComponent.SetHiddenInGame` (`/Game/Mods/AdminBooster/Blueprints/Buffs/Buff_ZomboSpeed.AdminTagBack` _asbuff_zombospeed_c) true false)
            (`SceneComponent.SetHiddenInGame` (`/Game/Mods/AdminBooster/Blueprints/Buffs/Buff_ZomboSpeed.AdminTagFront` _asbuff_zombospeed_c) true false))
          (:`then_3`
            (bind _returnvalue_5 (`PrimalCharacter.GetBuff` _asprimalcharacter "/Game/Mods/AdminBooster/Blueprints/Buffs/Buff_Speed.Buff_Speed_C"))
            (bind _asbuff_speed_c (cast `/Game/Mods/AdminBooster/Blueprints/Buffs/Buff_Speed` _returnvalue_5))
            (`SceneComponent.SetHiddenInGame` (`/Game/Mods/AdminBooster/Blueprints/Buffs/Buff_Speed.AdminTagBack` _asbuff_speed_c) true false)
            (`SceneComponent.SetHiddenInGame` (`/Game/Mods/AdminBooster/Blueprints/Buffs/Buff_Speed.AdminTagFront` _asbuff_speed_c) true false)))))))

(event `self.ReceiveDestroyed`
  ;[1 1 1] Buff Effects End
  (bind _asshootercharacter (cast `ShooterCharacter` (`self.Instigator`)))
  (`/Engine/EditorBlueprintResources/StandardMacros.IsValid` (`ShooterCharacter.CurrentWeapon` _asshootercharacter)
    (:`Is Valid`
      (`KismetSystemLibrary.ExecuteConsoleCommand` "cheat enemyinvisible false")
      (`KismetSystemLibrary.ExecuteConsoleCommand` "cheat setgodmode false")
      (bind _asprimalcharacter (cast `PrimalCharacter` (`self.GetOwner`)))
      (`|ExecutionSequence`
        (:`then_0`
          (bind _returnvalue (`PrimalCharacter.GetBuff` _asprimalcharacter "/Game/Mods/AdminBooster/Blueprints/Buffs/Buff_Vanish.Buff_Vanish_C"))
          (bind _asbuff_gm_c (cast `/GamingOGs Mods/AdminBooster/Blueprints/Buffs/Buff_GM` _returnvalue))
          (`SceneComponent.SetHiddenInGame` (`/GamingOGs Mods/AdminBooster/Blueprints/Buffs/Buff_GM.AdminTagBack` _asbuff_gm_c) false false)
          (`SceneComponent.SetHiddenInGame` (`/GamingOGs Mods/AdminBooster/Blueprints/Buffs/Buff_GM.AdminTagFront` _asbuff_gm_c) false false))
        (:`then_1`
          (bind _returnvalue_2 (`PrimalCharacter.GetBuff` _asprimalcharacter "/Game/Mods/AdminBooster/Blueprints/Buffs/Buff_Vanish.Buff_Vanish_C"))
          (bind _asbuff_zombogm_c (cast `/Game/Mods/AdminBooster/Blueprints/Buffs/Buff_ZomboGM` _returnvalue_2))
          (`SceneComponent.SetHiddenInGame` (`/Game/Mods/AdminBooster/Blueprints/Buffs/Buff_ZomboGM.AdminTagBack` _asbuff_zombogm_c) false false)
          (`SceneComponent.SetHiddenInGame` (`/Game/Mods/AdminBooster/Blueprints/Buffs/Buff_ZomboGM.AdminTagFront` _asbuff_zombogm_c) false false))
        (:`then_2`
          (bind _returnvalue_3 (`PrimalCharacter.GetBuff` _asprimalcharacter "/Game/Mods/AdminBooster/Blueprints/Buffs/Buff_Vanish.Buff_Vanish_C"))
          (bind _asbuff_zombospeed_c (cast `/Game/Mods/AdminBooster/Blueprints/Buffs/Buff_ZomboSpeed` _returnvalue_3))
          (`SceneComponent.SetHiddenInGame` (`/Game/Mods/AdminBooster/Blueprints/Buffs/Buff_ZomboSpeed.AdminTagBack` _asbuff_zombospeed_c) false false)
          (`SceneComponent.SetHiddenInGame` (`/Game/Mods/AdminBooster/Blueprints/Buffs/Buff_ZomboSpeed.AdminTagFront` _asbuff_zombospeed_c) false false))))))

(fn `UserConstructionScript`)