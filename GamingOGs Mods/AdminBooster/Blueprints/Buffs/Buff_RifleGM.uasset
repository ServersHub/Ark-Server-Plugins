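; Admin rifle buff that gives the instigating ShooterCharacter "leave me alone" cheat protection, implemented through console cheat commands.
; It sends leavemealone shortly after BeginPlay and again on every client buff tick, provided the character has a current weapon.
; On destruction, under the same weapon check, it switches off enemy invisibility and god mode and sends InfiniteStats without an argument.
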(event `self.BuffTickClient`
  (params (DeltaTime :type "Float (single-precision)"))
  (bind _instigator (`self.Instigator`))
  ;[1 1 1] Register Buff
  (`/Engine/EditorBlueprintResources/StandardMacros.IsValid` _instigator
    (:`Is Valid`
      (bind _asshootercharacter (cast `ShooterCharacter` _instigator))
      (`/Engine/EditorBlueprintResources/StandardMacros.IsValid` (`ShooterCharacter.CurrentWeapon` _asshootercharacter)
        (:`Is Valid`
          (`KismetSystemLibrary.ExecuteConsoleCommand` "cheat leavemealone"))))))

(event `self.ReceiveBeginPlay`
  ;[1 1 1] Give Buff
  (`KismetSystemLibrary.Delay` 0.2)
  (bind _asshootercharacter (cast `ShooterCharacter` (`self.Instigator`)))
  (`/Engine/EditorBlueprintResources/StandardMacros.IsValid` (`ShooterCharacter.CurrentWeapon` _asshootercharacter)
    (:`Is Valid`
      (`KismetSystemLibrary.ExecuteConsoleCommand` "cheat leavemealone"))))

(event `self.ReceiveDestroyed`
  ;[1 1 1] Destroy Buff
  (bind _asshootercharacter (cast `ShooterCharacter` (`self.Instigator`)))
  (`/Engine/EditorBlueprintResources/StandardMacros.IsValid` (`ShooterCharacter.CurrentWeapon` _asshootercharacter)
    (:`Is Valid`
      (`KismetSystemLibrary.ExecuteConsoleCommand` "cheat EnemyInvisible false")
      (`KismetSystemLibrary.ExecuteConsoleCommand` "cheat SetGodMode false")
      (`KismetSystemLibrary.ExecuteConsoleCommand` "cheat InfiniteStats"))))

(fn `UserConstructionScript`)