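; Admin buff from the AdminBooster mod that hides the player it is attached to for as long as it is active.
; Shortly after BeginPlay it hides the Instigator actor in game, and it unhides that actor when the buff is destroyed.
; The client buff tick, which must be enabled in the default settings, keeps hiding the character's current weapon; nothing here explicitly unhides the weapon.
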(event `self.BuffTickClient`
  (params (DeltaTime :type "Float (single-precision)"))
  (bind _instigator (`self.Instigator`))
  ;[1 1 1] ClientTick, needs to be set up in default settings
  ;[1 1 1] Check if we have a valid "player"
  (`/Engine/EditorBlueprintResources/StandardMacros.IsValid` _instigator
    (:`Is Valid`
      ;[1 1 1] Check if we have a valid weapon and hide
      (bind _asshootercharacter (cast `ShooterCharacter` _instigator))
      (bind _currentweapon (`ShooterCharacter.CurrentWeapon` _asshootercharacter))
      (`/Engine/EditorBlueprintResources/StandardMacros.IsValid` _currentweapon
        (:`Is Valid`
          (`self.SetActorHiddenInGame` _currentweapon true))))))

(event `self.ReceiveBeginPlay`
  ;[1 1 1] Begin Play
  (`KismetSystemLibrary.Delay` 0.2)
  ;[1 1 1] Hide the "player" actor
  (`self.SetActorHiddenInGame` (`self.Instigator`) true))

(event `self.ReceiveDestroyed`
  ;[1 1 1] Triggers when the buff is destroyed
  ;[1 1 1] Show the "player" actor
  (`self.SetActorHiddenInGame` (`self.Instigator`) false))

(fn `UserConstructionScript`)