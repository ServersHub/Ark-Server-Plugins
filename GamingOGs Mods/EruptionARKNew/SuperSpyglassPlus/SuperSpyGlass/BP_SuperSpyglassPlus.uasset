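; Super Spyglass Plus item that gives its holder adjustable zoom, a GPS widget and a target-lock toggle.
; On BeginPlay the local client enables input and shows the widget, while the server applies Buff_SuperSpyglassPlus; EndPlay removes the buff and toggles the widget off.
; Mouse wheel steps the targeting FOV within limits while aiming or riding.
; Fire calls a server event that relays the lock toggle through the buff.
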(event `self.ReceiveBeginPlay`
  (`KismetSystemLibrary.Delay` 0.2)
  (bind _returnvalue (`self.GetOwnerController`))
  (`|ExecutionSequence`
    (:`then_0`
      (if (`Controller.IsLocalController` _returnvalue)
        (`self.EnableInput` _returnvalue)
        (`self.Add GPS Widget` _returnvalue)))
    (:`then_1`
      (`/Engine/EditorBlueprintResources/ActorMacros.Switch Has Authority`
        (:`Authority`
          (bind _asshooterplayercontroller (cast `ShooterPlayerController` _returnvalue))
          (bind _returnvalue_2 (`PrimalBuff.StaticAddBuff` "/Game/Mods/EruptionARKNew/SuperSpyglassPlus/_Buffs/Buff_SuperSpyglassPlus.Buff_SuperSpyglassPlus_C" (`ShooterPlayerController.GetPlayerCharacter` _asshooterplayercontroller)))
          (bind _asbuff_superspyglassplus_c (cast `/Game/Mods/EruptionARKNew/SuperSpyglassPlus/_Buffs/Buff_SuperSpyglassPlus` _returnvalue_2))
          (set `self.BuffRef` _asbuff_superspyglassplus_c))))))

(event `self.ReceiveEndPlay`
  (params (EndPlayReason :type "EngineTypes.EEndPlayReason Enum" :default "ActorDestroyed"))
  (bind _buffref (`self.BuffRef`))
  (`/Engine/EditorBlueprintResources/ActorMacros.SwitchNetAuthority`
    (:`DedicatedServer`
      (`/Engine/EditorBlueprintResources/StandardMacros.IsValid` _buffref :!label _label
        (:`Is Valid`
          (`/Game/Mods/EruptionARKNew/SuperSpyglassPlus/_Buffs/Buff_SuperSpyglassPlus.ROS_RemoveBuff` _buffref))))
    (:`PlayerServer`
      (goto _label))
    (:`Client`
      (`self.Add GPS Widget` null))))

(event `InputAction|Targeting` :consume false :overrideparent false
  (:`Pressed`
    (set `self.IsRightMouseDown` true :!label _label_2))
  (:`Released`
    (set `self.IsRightMouseDown` false :!label _label_3)))

(event `InputAction|GamepadLeftFire` :consume false :overrideparent false
  (:`Pressed`
    (goto _label_2))
  (:`Released`
    (goto _label_3)))

(event `Key|MouseScrollUp` :consume false :overrideparent false
  (bind _overridetargetingfov (`self.OverrideTargetingFOV`))
  (:`Pressed`
    (bind _asshootercharacter (cast `ShooterCharacter` (`self.GetOwner`)))
    (if (`ShooterCharacter.bIsRiding` _asshootercharacter)
      (if (> _overridetargetingfov 10.0) :!label _label_4
        (set `self.OverrideTargetingFOV` (- _overridetargetingfov 5.0)))
      (elif (`self.IsRightMouseDown`)
        (goto _label_4)))))

(event `Key|MouseScrollDown` :consume false :overrideparent false
  (bind _overridetargetingfov (`self.OverrideTargetingFOV`))
  (:`Pressed`
    (bind _asshootercharacter (cast `ShooterCharacter` (`self.GetOwner`)))
    (if (`ShooterCharacter.bIsRiding` _asshootercharacter)
      (if (< _overridetargetingfov 90.0) :!label _label_5
        (set `self.OverrideTargetingFOV` (+ _overridetargetingfov 5.0)))
      (elif (`self.IsRightMouseDown`)
        (goto _label_5)))))

(event `InputAction|Fire`
  (:`Pressed`
    (`self.ROS_ToggleUILock` :!label _label_6)))

(event `InputAction|GamepadRightFire`
  (:`Pressed`
    (goto _label_6)))

(event `ROS_ToggleUILock`
  (bind _buffref (`self.BuffRef`))
  (`/Engine/EditorBlueprintResources/StandardMacros.IsValid` _buffref
    (:`Is Valid`
      (`/Game/Mods/EruptionARKNew/SuperSpyglassPlus/_Buffs/Buff_SuperSpyglassPlus.ROC_ToggleTargetLock` _buffref))))

(fn `Add GPS Widget`
  (params (LocalPC :type "PlayerController Object Reference"))
  (bind _gps_widget_ref (`self.GPS_Widget_Ref`))
  (`/Engine/EditorBlueprintResources/StandardMacros.IsValid` _gps_widget_ref
    (:`Is Valid`
      (`UserWidget.RemoveFromViewport` _gps_widget_ref)
      (set `self.GPS_Widget_Ref` null))
    (:`Is Not Valid`
      (bind _returnvalue (`|CreateWidget` "/Game/Mods/EruptionARKNew/SuperSpyglassPlus/_Widgets/GpsWidget_SSP.GpsWidget_SSP_C" LocalPC))
      (set `self.GPS_Widget_Ref` _returnvalue)
      (`UserWidget.AddToViewport` _returnvalue))))

(fn `UserConstructionScript`
  (`parent.UserConstructionScript`))