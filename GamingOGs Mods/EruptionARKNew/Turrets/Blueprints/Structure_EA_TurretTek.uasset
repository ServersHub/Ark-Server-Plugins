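; Tek turret structure for the Eruption mod that filters creature targets by a class include/exclude list and level range, with engram-gated access.
; Wheel menus offer nearby classes and level steps, sending client picks to the server as net exec commands.
; Turret-range limits, which also count Plant X seeded crop plots, block placement and deactivate excess turrets on save load, with HUD warnings.
; Targeting settings copy from other turrets.
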(fn ConstructionScript)

(fn BPGetMultiUseEntries
  (params (ForPC :type Player%20Controller%20Object%20Reference) (MultiUseEntries :type Array%20of%20Multi%20Use%20Entry%20Structures))
  (bind _returnvalue (Transformation|GetActorLocation))
  (bind _color (Math|Color|MakeColor 255 230 30 255))
  (bind _color_2 (Math|Color|MakeColor 220 255 30 255))
  (bind _color_3 (Math|Color|MakeColor 255 230 30 255))
  (bind _color_4 (Math|Color|MakeColor 255 230 30 255))
  (bind _color_5 (Math|Color|MakeColor 40 255 255 255))
  (bind _mindinolevel (Variables|Default|GetMinDinoLevel))
  (bind _maxdinolevel (Variables|Default|GetMaxDinoLevel))
  (bind _lastlocalinrangeclasses (Variables|Default|GetLastLocalInRangeClasses))
  (bind _bisinclusionlist (Variables|Default|GetbIsInclusionList))
  (bind _dinoclasslist (Variables|Default|GetDinoClassList))
  (Utilities|FlowControl|Sequence
    (:then_0
      (bind _asshooterplayercontroller (Utilities|Casting|CastToShooterPlayerController ForPC))
      (bind _returnvalue_2 (Class|PrimalStructure|AllowStructureAccess _asshooterplayercontroller))
      (if (and (== (Variables|/Script/Engine.Actor|GetTargetingTeam _asshooterplayercontroller) (Variables|Default|GetTargetingTeam)) _returnvalue_2)
        (Utilities|Array|Add MultiUseEntries (Utilities|Struct|MakeMultiUseEntry 0 (select _bisinclusionlist "Targeting: Inclusion List (Toggle)" "Targeting: Exclusion List (Toggle)") 55822 -11 false false false false false false false false true false false false false false 6))
        (if (Pawn|IsLocalPlayerController ForPC)
          (Utilities|Array|Add MultiUseEntries (Utilities|Struct|MakeMultiUseEntry 0 (select _bisinclusionlist "[Targeting: Add Nearby Creature Classes to Include]" "[Targeting: Add Nearby Creature Classes to Exclude]") 55820 -9 false false false false false false false false true true false true false false 6 "(B=175,G=175,R=175,A=255)" _color))
          (Utilities|Array|Add MultiUseEntries (Utilities|Struct|MakeMultiUseEntry 0 (select _bisinclusionlist "[Targeting: Remove Creature Classes to Include]" "[Targeting: Remove Creature Classes to Exclude]") 55821 -10 false false false false false false false false true true false true false false 6 "(B=175,G=175,R=175,A=255)" _color))
          (Utilities|Array|Add MultiUseEntries (Utilities|Struct|MakeMultiUseEntry 0 (Utilities|String|Append "[Set Minimum Creature Target Level" (select (> _mindinolevel 0) (Utilities|String|Append ": (" (Utilities|String|Append (Utilities|String|ToString(Integer) _mindinolevel) ")]")) "")) 55824 -6 false false false false false false false false true true false true false false 7 "(B=175,G=175,R=175,A=255)" _color_3))
          (Utilities|Array|Add MultiUseEntries (Utilities|Struct|MakeMultiUseEntry 0 (Utilities|String|Append "[Set Maximum Creature Target Level" (select (> _maxdinolevel 0) (Utilities|String|Append ": (" (Utilities|String|Append (Utilities|String|ToString(Integer) _maxdinolevel) ")]")) "")) 55825 -6 false false false false false false false false true true false true false false 7 "(B=175,G=175,R=175,A=255)" _color_3))
          (Utilities|Array|Add MultiUseEntries (Utilities|Struct|MakeMultiUseEntry 0 (select (Variables|Default|GetbIsInclusionList) "Leave 'Add to Inclusion List'" "Leave 'Add to Exclusion List'") 55826 10 false false false false false false false false true true false true false false 2 "(B=175,G=175,R=175,A=255)" _color_5))
          (Utilities|Array|Add MultiUseEntries (Utilities|Struct|MakeMultiUseEntry 0 (select (Variables|Default|GetbIsInclusionList) "Leave 'Remove from Inclusion List'" "Leave 'Remove from Exclusion List'") 55826 10 false false false false false false false false true true false true false false 3 "(B=175,G=175,R=175,A=255)" _color_5))
          (Utilities|Array|Add MultiUseEntries (Utilities|Struct|MakeMultiUseEntry 0 "Leave 'Minimum  Creature Level'" 55827 100 false false false false false false false false true true false true false false 4 "(B=175,G=175,R=175,A=255)" _color_5))
          (Utilities|Array|Add MultiUseEntries (Utilities|Struct|MakeMultiUseEntry 0 "Leave 'Maximum  Creature Level'" 55827 100 false false false false false false false false true true false true false false 5 "(B=175,G=175,R=175,A=255)" _color_5))
          (Utilities|Array|Add MultiUseEntries (Utilities|Struct|MakeMultiUseEntry 0 "[Set Targeting Options]" 55826 -9000 false false false false false false false false true true false true false false 0 "(B=175,G=175,R=175,A=255)" _color_4))
          (Utilities|Array|Add MultiUseEntries (Utilities|Struct|MakeMultiUseEntry 0 "[Set Creature Targeting Level Range]" 55827 -8000 false false false false false false false false true true false true false false 0 "(B=175,G=175,R=175,A=255)" _color_4))
          (Utilities|Array|Add MultiUseEntries (Utilities|Struct|MakeMultiUseEntry 0 "[Back]" 55823 1000000 false false false false false false false false true true false true false false 6 "(B=175,G=175,R=175,A=255)" _color_2))
          (Utilities|Array|Add MultiUseEntries (Utilities|Struct|MakeMultiUseEntry 0 "[Back]" 55823 1000000 false false false false false false false false true true false true false false 7 "(B=175,G=175,R=175,A=255)" _color_2))
          (Utilities|FlowControl|Sequence
            (:then_0
              (if (or (== (Variables|/Script/ShooterGame.ShooterPlayerController|GetViewingWheelCategory _asshooterplayercontroller) 3) (== (Variables|/Script/ShooterGame.ShooterPlayerController|GetViewingWheelCategory _asshooterplayercontroller) 2))
                (Utilities|Array|Clear _lastlocalinrangeclasses)
                (bind _outactors (Class|KismetSystemLibrary|SphereOverlapActorsNEW _returnvalue 6e+03 (Utilities|Array|MakeArray "ObjectTypeQuery7" "ObjectTypeQuery16")))
                (bind _returnvalue_3 (Class|VictoryCore|SortActorsbyDistance _returnvalue _outactors))
                (bind _array_element (Utilities|Array|ForEachLoopwithBreak _returnvalue_3 :!label _label)
                  (:LoopBody
                    (Utilities|FlowControl|Sequence
                      (:then_0
                        (bind _asprimaldinocharacter (Utilities|Casting|CastToPrimalDinoCharacter _array_element))
                        (bind _asprimaldinocharacter_2 (Utilities|Casting|CastToPrimalDinoCharacterClass (Utilities|GetClass _asprimaldinocharacter)))
                        (if (not (or (Utilities|Array|ContainsItem _dinoclasslist _asprimaldinocharacter_2) (Utilities|Array|ContainsItem _lastlocalinrangeclasses _asprimaldinocharacter_2)))
                          (Utilities|Array|Add _lastlocalinrangeclasses _asprimaldinocharacter_2)))
                      (:then_1
                        (if (>= (Utilities|Array|Length _lastlocalinrangeclasses) 16)
                          (goto _label Break)))))
                  (:Completed
                    (for (_array_element_2 _array_index) _lastlocalinrangeclasses
                      (bind _returnvalue_4 (Class|VictoryCore|GetClassDefaultObject _array_element_2))
                      (bind _asprimaldinocharacter_3 (Utilities|Casting|CastToPrimalDinoCharacter _returnvalue_4))
                      (Utilities|Array|Add MultiUseEntries (Utilities|Struct|MakeMultiUseEntry 0 (Variables|/Script/ShooterGame.PrimalCharacter|GetDescriptiveName _asprimaldinocharacter_3) (+ _array_index 56000) 0 false false false false false false false false true false false true false false 2)))
                    (for (_array_element_3 _array_index_2) _dinoclasslist
                      (bind _returnvalue_5 (Class|VictoryCore|GetClassDefaultObject _array_element_3))
                      (bind _asprimaldinocharacter_4 (Utilities|Casting|CastToPrimalDinoCharacter _returnvalue_5))
                      (Utilities|Array|Add MultiUseEntries (Utilities|Struct|MakeMultiUseEntry 0 (Variables|/Script/ShooterGame.PrimalCharacter|GetDescriptiveName _asprimaldinocharacter_4) (+ _array_index_2 57000) 0 false false false false false false false false true false false true false false 3)))))))
            (:then_1
              (if (or (== (Variables|/Script/ShooterGame.ShooterPlayerController|GetViewingWheelCategory _asshooterplayercontroller) 4) (== (Variables|/Script/ShooterGame.ShooterPlayerController|GetViewingWheelCategory _asshooterplayercontroller) 5))
                (for _index (range 0 20)
                  (Utilities|Array|Add MultiUseEntries (Utilities|Struct|MakeMultiUseEntry 0 (Utilities|Select :Index _index :Option%200 "Clear" :Option%201 "20" :Option%202 "40" :Option%203 "60" :Option%204 "80" :Option%205 "100" :Option%206 "120" :Option%207 "140" :Option%208 "160" :Option%209 "180" :Option%2010 "200" :Option%2011 "220" :Option%2012 "240" :Option%2013 "260" :Option%2014 "280" :Option%2015 "300" :Option%2016 "320" :Option%2017 "340" :Option%2018 "360" :Option%2019 "380" :Option%2020 "400") (+ _index 58100) (* _index -1) false false false false false false false false false false false true false false 4))
                  (Utilities|Array|Add MultiUseEntries (Utilities|Struct|MakeMultiUseEntry 0 (Utilities|Select :Index _index :Option%200 "Clear" :Option%201 "20" :Option%202 "40" :Option%203 "60" :Option%204 "80" :Option%205 "100" :Option%206 "120" :Option%207 "140" :Option%208 "160" :Option%209 "180" :Option%2010 "200" :Option%2011 "220" :Option%2012 "240" :Option%2013 "260" :Option%2014 "280" :Option%2015 "300" :Option%2016 "320" :Option%2017 "340" :Option%2018 "360" :Option%2019 "380" :Option%2020 "400") (+ _index 58200) (* _index -1) false false false false false false false false false false false true false false 5)))))))))
    (:then_1
      (return MultiUseEntries))))

(fn BPTryMultiUse
  (params (ForPC :type Player%20Controller%20Object%20Reference) (UseIndex :type Integer))
  (Utilities|FlowControl|Sequence
    (:then_0
      (switch int UseIndex
        (:55822
          (Variables|Default|SetbIsInclusionList (not (Variables|Default|GetbIsInclusionList)) true))))
    (:then_1
      (return true))))

(fn BPClientDoMultiUse
  (params (ForPC :type Player%20Controller%20Object%20Reference) (ClientUseIndex :type Integer))
  (bind _returnvalue (- ClientUseIndex 56000))
  (bind _returnvalue_2 (- ClientUseIndex 57000))
  (bind _self self)
  (bind _lastlocalinrangeclasses (Variables|Default|GetLastLocalInRangeClasses))
  (bind _dinoclasslist (Variables|Default|GetDinoClassList))
  (bind _item (Utilities|Array|Get(acopy) _lastlocalinrangeclasses _returnvalue))
  (bind _item_2 (Utilities|Array|Get(acopy) _dinoclasslist _returnvalue_2))
  (bind _asshooterplayercontroller (Utilities|Casting|CastToShooterPlayerController ForPC))
  (switch int ClientUseIndex
    (:Default
      (if (and (>= ClientUseIndex 56000) (< ClientUseIndex 57000))
        (if (!= _item 0)
          (bind _returnvalue_3 (Class|VictoryCore|GetClassDefaultObject _item))
          (bind _asprimaldinocharacter (Utilities|Casting|CastToPrimalDinoCharacter _returnvalue_3))
          (Class|PlayerController|ClientSendNetExecCommandtoServer _asshooterplayercontroller _self "Add" (Utilities|Struct|MakeBPNetExecParams 0 0 0 0.0 0.0 0.0 _asprimaldinocharacter) true))
        (elif (and (>= ClientUseIndex 57000) (< ClientUseIndex 58000))
          (if (!= _item_2 0)
            (bind _returnvalue_4 (Class|VictoryCore|GetClassDefaultObject _item_2))
            (bind _asprimaldinocharacter_2 (Utilities|Casting|CastToPrimalDinoCharacter _returnvalue_4))
            (Class|PlayerController|ClientSendNetExecCommandtoServer _asshooterplayercontroller _self "Remove" (Utilities|Struct|MakeBPNetExecParams 0 0 0 0.0 0.0 0.0 _asprimaldinocharacter_2) true))
          (elif (and (>= ClientUseIndex 58100) (< ClientUseIndex 58200))
            (Class|PlayerController|ClientSendNetExecCommandtoServer _asshooterplayercontroller _self "MinLevel" (Utilities|Struct|MakeBPNetExecParams (- ClientUseIndex 58100)) true)
            (elif (and (>= ClientUseIndex 58200) (< ClientUseIndex 58300))
              (Class|PlayerController|ClientSendNetExecCommandtoServer _asshooterplayercontroller _self "MaxLevel" (Utilities|Struct|MakeBPNetExecParams (- ClientUseIndex 58200)) true))))))
    (:55820
      (Class|ShooterPlayerController|SetMultiUseWheelCategory _asshooterplayercontroller 2))
    (:55821
      (Class|ShooterPlayerController|SetMultiUseWheelCategory _asshooterplayercontroller 3))
    (:55823
      (Class|ShooterPlayerController|SetMultiUseWheelCategory _asshooterplayercontroller 0))
    (:55824
      (Class|ShooterPlayerController|SetMultiUseWheelCategory _asshooterplayercontroller 4))
    (:55825
      (Class|ShooterPlayerController|SetMultiUseWheelCategory _asshooterplayercontroller 5))
    (:55826
      (Class|ShooterPlayerController|SetMultiUseWheelCategory _asshooterplayercontroller 6))
    (:55827
      (Class|ShooterPlayerController|SetMultiUseWheelCategory _asshooterplayercontroller 7))))

(fn BPServerHandleNetExecCommand
  (params (FromPC :type Player%20Controller%20Object%20Reference) (CommandName :type Name :default "None") (ExecParams :type BP%20Net%20Exec%20Params%20Structure%20%28by%20ref%29))
  (bind (_intparam1 _intparam2 _intparam3 _floatparam1 _floatparam2 _floatparam3 _objparam1) (Utilities|Struct|BreakBPNetExecParams ExecParams))
  (bind _returnvalue (Utilities|GetClass _objparam1))
  (bind _returnvalue_2 (Math|Integer|Clamp(Integer) _intparam1 0 20))
  (bind _returnvalue_3 (* _returnvalue_2 20))
  (Utilities|FlowControl|Sequence
    (:then_0
      (bind _asshooterplayercontroller (Utilities|Casting|CastToShooterPlayerController FromPC))
      (bind _returnvalue_4 (Class|PrimalStructure|AllowStructureAccess _asshooterplayercontroller))
      (if (and (== (Variables|/Script/Engine.Actor|GetTargetingTeam FromPC) (Variables|Default|GetTargetingTeam)) _returnvalue_4)
        (switch name CommandName
          (:Add
            (bind _asprimaldinocharacter (Utilities|Casting|CastToPrimalDinoCharacterClass _returnvalue))
            (LocalVariables|SetNewArray (Variables|Default|GetDinoClassList))
            (if (and (< (Utilities|Array|Length (Variables|Default|GetDinoClassList)) (Variables|Default|GetMaxDinoClasses)) (not (Utilities|Array|ContainsItem (Variables|Default|GetDinoClassList) _asprimaldinocharacter)))
              (Utilities|Array|Add (LocalVariables|GetNewArray) _asprimaldinocharacter)
              (Variables|Default|SetDinoClassList (LocalVariables|GetNewArray) true :!label _label)))
          (:Remove
            (bind _asprimaldinocharacter_2 (Utilities|Casting|CastToPrimalDinoCharacterClass _returnvalue))
            (LocalVariables|SetNewArray (Variables|Default|GetDinoClassList))
            (if (Utilities|Array|ContainsItem (Variables|Default|GetDinoClassList) _asprimaldinocharacter_2)
              (Utilities|Array|RemoveItem (LocalVariables|GetNewArray) _asprimaldinocharacter_2)
              (goto _label)))
          (:MinLevel
            (Variables|Default|SetMinDinoLevel _returnvalue_3 true))
          (:MaxLevel
            (Variables|Default|SetMaxDinoLevel _returnvalue_3 true)))))
    (:then_1
      (return true))))

(fn BPTurretPreventsTargeting
  (params (PotentialTarget :type Primal%20Character%20Object%20Reference))
  (bind _mindinolevel (Variables|Default|GetMinDinoLevel))
  (bind _maxdinolevel (Variables|Default|GetMaxDinoLevel))
  (bind _bisinclusionlist (Variables|Default|GetbIsInclusionList))
  (Utilities|FlowControl|Sequence
    (:then_0
      (if (Class|Actor|IsPrimalDino PotentialTarget)
        (bind _asprimaldinocharacter (Utilities|Casting|CastToPrimalDinoCharacterClass (Utilities|GetClass PotentialTarget)))
        (Utilities|FlowControl|Sequence
          (:then_0
            (if (Utilities|Array|ContainsItem (Variables|Default|GetDinoClassList) _asprimaldinocharacter)
              (LocalVariables|SetbRetVal (not _bisinclusionlist))
              (else
                (LocalVariables|SetbRetVal _bisinclusionlist))))
          (:then_1
            (if (and (not (LocalVariables|GetbRetVal)) (> (+ _maxdinolevel _mindinolevel) 0))
              (bind _asprimaldinocharacter_2 (Utilities|Casting|CastToPrimalDinoCharacter PotentialTarget))
              (Utilities|FlowControl|Sequence
                (:then_0
                  (if (< (Class|PrimalCharacterStatusComponent|GetCharacterLevel (Variables|/Script/ShooterGame.PrimalCharacter|GetMyCharacterStatusComponent _asprimaldinocharacter_2)) _mindinolevel)
                    (LocalVariables|SetbRetVal true)))
                (:then_1
                  (if (and (> _maxdinolevel 0) (> (Class|PrimalCharacterStatusComponent|GetCharacterLevel (Variables|/Script/ShooterGame.PrimalCharacter|GetMyCharacterStatusComponent _asprimaldinocharacter_2)) _maxdinolevel))
                    (LocalVariables|SetbRetVal true)))))))))
    (:then_1
      (return (LocalVariables|GetbRetVal)))))

(fn BPOverrideAllowStructureAccess
  (params (ForPC :type Shooter%20Player%20Controller%20Object%20Reference) (bIsAccessAllowed :type Boolean) (bForInventoryOnly :type Boolean))
  (bind _playerstate (Variables|/Script/Engine.Controller|GetPlayerState ForPC))
  (LocalVariables|SetbRetVal bIsAccessAllowed)
  (Utilities|FlowControl|Sequence
    (:then_0
      (if (LocalVariables|GetbRetVal)
        (bind _asshooterplayerstate (Utilities|Casting|CastToShooterPlayerState _playerstate))
        (bind _returnvalue (Class|ShooterPlayerController|AllowTribeGroupPermission ForPC "STRUCTUREACTIVATE" self))
        (LocalVariables|SetbRetVal (Math|Boolean|ANDBoolean (Class|ShooterPlayerState|HasEngram _asshooterplayerstate (Variables|Default|GetPickupGivesItem)) bIsAccessAllowed _returnvalue))))
    (:then_1
      (if (Class|VictoryCore|IsTimeSinceNetwork (Class|Actor|GetWorld) (Variables|Default|GetLastTimePrintDebugString) 5.0 true)
        (bind _asshooterplayerstate_2 (Utilities|Casting|CastToShooterPlayerState _playerstate))))
    (:then_2
      (return (or (LocalVariables|GetbRetVal) bForInventoryOnly)))))

(fn BPCanbeActivatedbyPlayer
  (params (PC :type Shooter%20Player%20Controller%20Object%20Reference))
  (bind _returnvalue (Class|PrimalStructure|AllowStructureAccess PC))
  (return _returnvalue))

(fn BlueprintDrawHUD
  (params (HUD :type Shooter%20HUD%20Object%20Reference) (CenterX :type Float%20%28single-precision%29) (CenterY :type Float%20%28single-precision%29))
  (bind _color (Math|Color|MakeColor 0 0 255 255))
  (bind _canvas (Variables|/Script/Engine.HUD|GetCanvas HUD))
  (bind _normalfont (Variables|/Script/ShooterGame.ShooterHUD|GetNormalFont HUD))
  (bind _canvas_2 (Variables|/Script/Engine.HUD|GetCanvas HUD))
  (if (Variables|Default|GetbTooManyInRangeInactive)
    (Class|Canvas|SetDrawColor _canvas (Math|Color|MakeColor 0 0 255 255))
    (Class|Canvas|BPDrawTextCentered _canvas (Variables|/Script/ShooterGame.ShooterHUD|GetNormalFont HUD) "INACTIVE DUE TO TOO MANY TURRETS IN RANGE! RE-PLACE THIS TURRET!" CenterX (- CenterY 1.2e+02) 1.0 1.0 true true))
  (bind _asshootergamestate (Utilities|Casting|CastToShooterGameState (Game|GetGameState)))
  (if (Variables|/Script/ShooterGame.ShooterGameState|GetbLimitTurretsInRange _asshootergamestate)
    (if (== (Variables|/Script/Engine.Actor|GetTargetingTeam (Class|ShooterHUD|GetShooterPC HUD)) (Variables|Default|GetTargetingTeam))
      (bind _returnvalue (Class|PrimalStructure|GetNumStructuresinRangeStructureTypeFlag (Class|Actor|GetWorld) (Transformation|GetActorLocation) 262144 (Variables|/Script/ShooterGame.ShooterGameState|GetLimitTurretsRange _asshootergamestate) false false 0 false))
      (if (> _returnvalue (Variables|/Script/ShooterGame.ShooterGameState|GetLimitTurretsNum _asshootergamestate))
        (Class|Canvas|SetDrawColor _canvas_2 _color)
        (else
          (Class|Canvas|SetDrawColor _canvas_2 (Math|Color|MakeColor 0 255 0 255))))
      (Class|Canvas|BPDrawTextCentered _canvas_2 _normalfont (Utilities|String|ToString(Text) (Utilities|Text|FormatText "Turrets In Range {0} / {1}" (Utilities|Text|ToText(Integer) _returnvalue) (Utilities|Text|ToText(Integer) (Variables|/Script/ShooterGame.ShooterGameState|GetLimitTurretsNum _asshootergamestate)))) CenterX (- CenterY 8e+01) 1.0 1.0 true true)
      (if (> _returnvalue (Variables|/Script/ShooterGame.ShooterGameState|GetLimitTurretsNum _asshootergamestate))
        (Class|Canvas|SetDrawColor _canvas_2 _color)
        (Class|Canvas|BPDrawTextCentered _canvas_2 _normalfont "Too many Turrets in range! Move Turrets to retain functionality!" CenterX (- CenterY 1e+02) 1.0 1.0 true true)))))

(fn BPIsAllowedtoBuildEx
  (params (OutPlacementData :type Placement%20Data%20Structure%20%28by%20ref%29) (CurrentAllowedReason :type Integer) (PC :type Player%20Controller%20Object%20Reference) (bFinalPlacement :type Boolean) (bChoosingRotation :type Boolean))
  (bind _adjustedlocation (Utilities|Struct|BreakPlacementData OutPlacementData))
  (bind _returnvalue (Class|Actor|GetWorld))
  (LocalVariables|SetbRetVal true)
  (bind _asshootergamestate (Utilities|Casting|CastToShooterGameState (Game|GetGameState)))
  (bind _asprimalworldsettings (Utilities|Casting|CastToPrimalWorldSettings (Class|World|GetWorldSettings (Class|Actor|GetWorld) false true)))
  (if (and (Variables|/Script/ShooterGame.ShooterGameState|GetbLimitTurretsInRange _asshootergamestate) true)
    (Utilities|FlowControl|Sequence
      (:then_0
        (Utilities|FlowControl|Sequence
          (:then_0
            (bind _returnvalue_2 (Class|PrimalStructure|GetNumStructuresinRangeStructureTypeFlag _returnvalue _adjustedlocation 262144 (Variables|/Script/ShooterGame.ShooterGameState|GetLimitTurretsRange _asshootergamestate) false false 0 false))
            (LocalVariables|SetNumTurrets _returnvalue_2)
            (if (Networking|IsServer)
              (bind _structuresout (Class|PrimalStructure|GetStructuresinRange _returnvalue _adjustedlocation (Variables|/Script/ShooterGame.ShooterGameState|GetLimitTurretsRange _asshootergamestate) "/Game/PrimalEarth/Structures/BuildingBases/CropPlotBaseBP.CropPlotBaseBP_C" false))
              (for _array_element _structuresout
                (bind _asprimalstructureitemcontainer_cropplot (Utilities|Casting|CastToPrimalStructureItemContainer_CropPlot _array_element))
                (Utilities|Casting|CastToPrimalStructureTurret (Variables|/Script/ShooterGame.PrimalStructureItemContainer_CropPlot|GetMyCropStructure _asprimalstructureitemcontainer_cropplot)
                  (:CastFailed
                    (bind _returnvalue_3 (Class|PrimalInventoryComponent|GetItemTemplateQuantity (Variables|/Script/ShooterGame.PrimalStructureItemContainer|GetMyInventoryComponent _asprimalstructureitemcontainer_cropplot) "/Game/PrimalEarth/CoreBlueprints/Items/Consumables/Seeds/PrimalItemConsumable_Seed_DefensePlant.PrimalItemConsumable_Seed_DefensePlant_C" 0 true false false false))
                    (if (or (> _returnvalue_3 0) (Utilities|ClassIsChildOf (Variables|/Script/ShooterGame.PrimalStructureItemContainer_CropPlot|GetPlantedCrop _asprimalstructureitemcontainer_cropplot) "/Game/PrimalEarth/CoreBlueprints/Items/Consumables/Seeds/PrimalItemConsumable_Seed_DefensePlant.PrimalItemConsumable_Seed_DefensePlant_C"))
                      (LocalVariables|SetNumTurrets (+ (LocalVariables|GetNumTurrets) 1))))))))
          (:then_1
            (if (>= (LocalVariables|GetNumTurrets) (Variables|/Script/ShooterGame.ShooterGameState|GetLimitTurretsNum _asshootergamestate))
              (LocalVariables|SetbRetVal false)))))
      (:then_1
        (if (Pawn|IsLocalPlayerController PC)
          _
          (else
            _))
        (bind _asshooterplayercontroller (Utilities|Casting|CastToShooterPlayerController PC))
        (Class|ShooterPlayerController|ClientHUDNotificationTypeParams _asshooterplayercontroller (Math|Integer|SelectInt 1010836 1010835 (LocalVariables|GetbRetVal)) (LocalVariables|GetNumTurrets) (Variables|/Script/ShooterGame.ShooterGameState|GetLimitTurretsNum _asshootergamestate) (Class|VictoryCore|ClassReftoObjectRef (Utilities|GetClass self))))
      (:then_2
        (return (Math|Integer|SelectInt CurrentAllowedReason -15 (LocalVariables|GetbRetVal)))))
    (else
      (return (Math|Integer|SelectInt CurrentAllowedReason -15 (LocalVariables|GetbRetVal))))))

(fn BPPostLoadedfromSaveGame
  (CallFunction|TurretCheckHardLimit))

(fn TurretCheckHardLimit
  (bind _returnvalue (Class|Actor|GetWorld))
  (bind _returnvalue_2 (Transformation|GetActorLocation))
  (bind _self self)
  (bind _asshootergamemode (Utilities|Casting|CastToShooterGameMode (Game|GetGameMode)))
  (if (Variables|/Script/ShooterGame.ShooterGameMode|GetbHardLimitTurretsInRange _asshootergamemode)
    (Utilities|FlowControl|Sequence
      (:then_0
        (bind _returnvalue_3 (Class|PrimalStructure|GetNumStructuresinRangeStructureTypeFlag _returnvalue _returnvalue_2 262144 (Variables|/Script/ShooterGame.ShooterGameMode|GetLimitTurretsRange _asshootergamemode) true true _self false))
        (LocalVariables|SetNumTurrets _returnvalue_3)
        (if (Networking|IsServer)
          (bind _structuresout (Class|PrimalStructure|GetStructuresinRange _returnvalue _returnvalue_2 (Variables|/Script/ShooterGame.ShooterGameMode|GetLimitTurretsRange _asshootergamemode) "/Game/PrimalEarth/Structures/BuildingBases/CropPlotBaseBP.CropPlotBaseBP_C" true _self))
          (for _array_element _structuresout
            (bind _asprimalstructureitemcontainer_cropplot (Utilities|Casting|CastToPrimalStructureItemContainer_CropPlot _array_element))
            (Utilities|Casting|CastToPrimalStructureTurret (Variables|/Script/ShooterGame.PrimalStructureItemContainer_CropPlot|GetMyCropStructure _asprimalstructureitemcontainer_cropplot)
              (:CastFailed
                (bind _returnvalue_4 (Class|PrimalInventoryComponent|GetItemTemplateQuantity (Variables|/Script/ShooterGame.PrimalStructureItemContainer|GetMyInventoryComponent _asprimalstructureitemcontainer_cropplot) "/Game/PrimalEarth/CoreBlueprints/Items/Consumables/Seeds/PrimalItemConsumable_Seed_DefensePlant.PrimalItemConsumable_Seed_DefensePlant_C" 0 true false false false))
                (if (or (> _returnvalue_4 0) (Utilities|ClassIsChildOf (Variables|/Script/ShooterGame.PrimalStructureItemContainer_CropPlot|GetPlantedCrop _asprimalstructureitemcontainer_cropplot) "/Game/PrimalEarth/CoreBlueprints/Items/Consumables/Seeds/PrimalItemConsumable_Seed_DefensePlant.PrimalItemConsumable_Seed_DefensePlant_C"))
                  (LocalVariables|SetNumTurrets (+ (LocalVariables|GetNumTurrets) 1))))))))
      (:then_1
        (if (>= (LocalVariables|GetNumTurrets) (Variables|/Script/ShooterGame.ShooterGameMode|GetLimitTurretsNum _asshootergamemode))
          (Variables|Default|SetbTooManyInRangeInactive true false)
          (if (Variables|Default|GetbContainerActivated)
            (Class|PrimalStructure|SetContainerActive false))
          (else
            (Variables|Default|SetbTooManyInRangeInactive false false)))))))

(fn BPCanbeActivated
  (return (not (Variables|Default|GetbTooManyInRangeInactive))))

(fn BPCopyCustomSettingsfromTurret
  (params (FromTurret :type Primal%20Structure%20Turret%20Object%20Reference))
  (Utilities|FlowControl|Sequence
    (:then_0
      (bind _asstructureturrettek_c (Utilities|Casting|CastToStructureTurretTek FromTurret)
        (:then
          (Variables|Default|SetbIsInclusionList (Variables|/Game/PrimalEarth/Structures/BuildingBases/StructureTurretTek.StructureTurretTek_C|GetbIsInclusionList _asstructureturrettek_c) false)
          (Variables|Default|SetDinoClassList (Variables|/Game/PrimalEarth/Structures/BuildingBases/StructureTurretTek.StructureTurretTek_C|GetDinoClassList _asstructureturrettek_c) false)
          (Variables|Default|SetMaxDinoLevel (Variables|/Game/PrimalEarth/Structures/BuildingBases/StructureTurretTek.StructureTurretTek_C|GetMaxDinoLevel _asstructureturrettek_c) false)
          (Variables|Default|SetMinDinoLevel (Variables|/Game/PrimalEarth/Structures/BuildingBases/StructureTurretTek.StructureTurretTek_C|GetMinDinoLevel _asstructureturrettek_c) false))
        (:CastFailed
          (bind _asstructureturretbasebp_baseheavy_c (Utilities|Casting|CastToStructureTurretBaseBP_BaseHeavy FromTurret)
            (:then
              (Variables|Default|SetbIsInclusionList (Variables|/Game/PrimalEarth/Structures/BuildingBases/StructureTurretBaseBP_BaseHeavy.StructureTurretBaseBP_BaseHeavy_C|GetbIsInclusionList _asstructureturretbasebp_baseheavy_c) false)
              (Variables|Default|SetDinoClassList (Variables|/Game/PrimalEarth/Structures/BuildingBases/StructureTurretBaseBP_BaseHeavy.StructureTurretBaseBP_BaseHeavy_C|GetDinoClassList _asstructureturretbasebp_baseheavy_c) false))
            (:CastFailed
              (bind _asstructureturretbasebp_c (Utilities|Casting|CastToStructureTurretBaseBP FromTurret))
              (Variables|Default|SetbIsInclusionList (Variables|/Game/PrimalEarth/Structures/BuildingBases/StructureTurretBaseBP.StructureTurretBaseBP_C|GetbIsInclusionList _asstructureturretbasebp_c) false)
              (Variables|Default|SetDinoClassList (Variables|/Game/PrimalEarth/Structures/BuildingBases/StructureTurretBaseBP.StructureTurretBaseBP_C|GetDinoClassList _asstructureturretbasebp_c) false))))))
    (:then_1
      (return true))))