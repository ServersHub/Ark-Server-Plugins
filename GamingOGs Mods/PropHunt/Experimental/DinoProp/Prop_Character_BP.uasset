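; Prop Hunt character (experimental dino-based) that takes on the look of a prop and can carry a rider.
; The replicated Prop struct sets the static mesh, offset and scale through its OnRep, which the construction script also calls.
; With a valid rider, incoming damage is re-applied to the rider as human melee damage and zeroed on the prop.
; It also blocks cryo, fall damage and damage impulses.
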(fn `BPAdjustDamage`
  (params (IncomingDamage :type "Float (double-precision)") (TheDamageEvent :type "EngineTypes.DamageEvent Structure") (EventInstigator :type "Controller Object Reference") (DamageCauser :type "Actor Object Reference") (bIsPointDamage :type Boolean) (PointHitInfo :type "EngineTypes.HitResult Structure"))
  (returns (ReturnValue :type "Float (double-precision)"))
  (bind _rider (`self.Rider`))
  (`/Engine/EditorBlueprintResources/StandardMacros.IsValid` _rider
    (:`Is Valid`
      (`GameplayStatics.ApplyDamage` _rider IncomingDamage EventInstigator DamageCauser "/Game/PrimalEarth/CoreBlueprints/DamageTypes/DmgType_Melee_Human.DmgType_Melee_Human_C")
      (return 0.0))))

(fn `BPAdjustImpulseFromDamage`
  (params (DesiredImpulse :type "Object.Vector Structure") (DamageTaken :type "Float (double-precision)") (TheDamageEvent :type "EngineTypes.DamageEvent Structure") (PawnInstigator :type "Pawn Object Reference") (DamageCauser :type "Actor Object Reference") (bIsPointDamage :type Boolean) (PointHitInfo :type "EngineTypes.HitResult Structure"))
  (returns (ReturnValue :type "Object.Vector Structure"))
  (return (0.0 0.0 0.0)))

(fn `BPCanCryo`
  (params (ForPC :type "ShooterPlayerController Object Reference"))
  (returns (ReturnValue :type Boolean))
  (return false))

(fn `BPPreventFallDamage`
  (params (HitResult :type "EngineTypes.HitResult Structure (by ref)") (FallDamageAmount :type "Float (double-precision)"))
  (returns (ReturnValue :type Boolean))
  (return true))

(fn `OnRep_Prop`
  (bind _staticmesh (`self.StaticMesh`))
  (bind ((`Mesh_3_AA2D810B4A6D9036D2410785A4AFD10F` _mesh) (`Offset_6_99D67ADF4B56DBF60883928A4E1EDE81` _offset) (`Scale_13_8443FF8942C46CCD17787394A3013A8F` _scale)) (break `/Game/Mods/HideAndSeek/Structs/PropStruct` (`self.Prop`)))
  (`StaticMeshComponent.SetStaticMesh` _staticmesh _mesh)
  (`SceneComponent.SetRelativeLocation` _staticmesh _offset false)
  (`SceneComponent.SetRelativeScale3D` _staticmesh _scale))

(fn `UserConstructionScript`
  (`parent.UserConstructionScript`)
  (`self.OnRep_Prop`))