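; Base buff Blueprint for the UpdatedMark mod that puts a UI widget on the owning player's screen while the buff is active.
; Ten seconds after BeginPlay, on a player server or client, it creates Widget_BP_UI for the owner controller, if valid, and adds it to the viewport.
; When the buff deactivates, it removes the stored widget from the viewport.
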(event `self.ReceiveBeginPlay`
  (`KismetSystemLibrary.Delay` 10.0)
  (`/Engine/EditorBlueprintResources/ActorMacros.SwitchNetAuthority`
    (:`PlayerServer`
      _)
    (:`Client`
      _))
  (bind _returnvalue (`self.GetOwnerController`))
  (`/Engine/EditorBlueprintResources/StandardMacros.IsValid` _returnvalue
    (:`Is Valid`
      (bind _returnvalue_2 (`|CreateWidget` "/Game/Mods/UpdatedMark/Widgets/Widget_BP_UI.Widget_BP_UI_C" _returnvalue))
      (set `self.Widget_UI` _returnvalue_2)
      (`UserWidget.AddToViewport` _returnvalue_2))))

(event `self.BPDeactivated`
  (params (ForInstigator :type "Actor Object Reference"))
  (bind _widget_ui (`self.Widget_UI`))
  (`/Engine/EditorBlueprintResources/StandardMacros.IsValid` _widget_ui
    (:`Is Valid`
      (`UserWidget.RemoveFromViewport` _widget_ui))))

(fn `UserConstructionScript`)